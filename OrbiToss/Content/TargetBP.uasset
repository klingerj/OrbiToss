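; TargetBP is a target that shows whether it has been hit through the material on its Cylinder mesh.
; Every Tick it reads BeenHit and assigns either the TargetHit or TargetMat material to slot 0; nothing in this file sets that flag.
; Two disconnected nodes that would set a red or green "color" vector parameter never run, and the construction script is empty.
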(event `self.ReceiveTick`
  (params (DeltaSeconds :type "Float (single-precision)"))
  (if (`self.beenHit`)
    (`PrimitiveComponent.SetMaterial` (`self.Cylinder`) 0 "/Game/Materials/TargetHit.TargetHit")
    (else
      (`PrimitiveComponent.SetMaterial` (`self.Cylinder`) 0 "/Game/Materials/TargetMat.TargetMat"))))

(fn `UserConstructionScript`)
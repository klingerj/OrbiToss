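; Level manager actor that records completion of three levels in GiuseppesGameInstance.
; Every Tick it checks its LevelComplete flags and sets the matching flags on the game instance.
; It enables input on BeginPlay, with shortcut actions that mark a level complete and open VR_Level_Selection.
; Another input action, StartLevel1, opens the VRTestSPANCER map directly.
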(event `self.ReceiveBeginPlay`
  (`self.EnableInput` (`GameplayStatics.GetPlayerController` 0)))

(event `self.ReceiveTick`
  (params (DeltaSeconds :type "Float (single-precision)"))
  (if (`self.level1Complete`)
    (bind _asgiuseppes_game_instance (cast `/Game/GiuseppesGameInstance` (`GameplayStatics.GetGameInstance`)))
    (set `/Game/GiuseppesGameInstance.Level1Complete` true _asgiuseppes_game_instance))
  (if (`self.level2Complete`)
    (bind _asgiuseppes_game_instance_2 (cast `/Game/GiuseppesGameInstance` (`GameplayStatics.GetGameInstance`)))
    (set `/Game/GiuseppesGameInstance.Level2Complete` true _asgiuseppes_game_instance_2))
  (if (`self.level3Complete`)
    (bind _asgiuseppes_game_instance_3 (cast `/Game/GiuseppesGameInstance` (`GameplayStatics.GetGameInstance`)))
    (set `/Game/GiuseppesGameInstance.Level3Complete` true _asgiuseppes_game_instance_3)))

(event `InputAction|AutoCompleteLevel1`
  (params (Key :type "Key Structure"))
  (:`Pressed`
    (bind _asgiuseppes_game_instance (cast `/Game/GiuseppesGameInstance` (`GameplayStatics.GetGameInstance`)))
    (set `/Game/GiuseppesGameInstance.Level1Complete` true _asgiuseppes_game_instance)
    (`GameplayStatics.OpenLevel` "VR_Level_Selection")))

(event `InputAction|AutoCompleteLevel2`
  (params (Key :type "Key Structure"))
  (:`Pressed`
    (bind _asgiuseppes_game_instance (cast `/Game/GiuseppesGameInstance` (`GameplayStatics.GetGameInstance`)))
    (set `/Game/GiuseppesGameInstance.Level2Complete` true _asgiuseppes_game_instance)
    (`GameplayStatics.OpenLevel` "VR_Level_Selection")))

(event `InputAction|AutoCompleteLevel3`
  (params (Key :type "Key Structure"))
  (:`Pressed`
    (bind _asgiuseppes_game_instance (cast `/Game/GiuseppesGameInstance` (`GameplayStatics.GetGameInstance`)))
    (set `/Game/GiuseppesGameInstance.Level3Complete` true _asgiuseppes_game_instance)
    (`GameplayStatics.OpenLevel` "VR_Level_Selection")))

(event `InputAction|StartLevel1`
  (params (Key :type "Key Structure"))
  (:`Pressed`
    (`GameplayStatics.OpenLevel` "VRTestSPANCER")))

(fn `UserConstructionScript`)
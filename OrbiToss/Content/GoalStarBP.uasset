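; GoalStarBP is a goal star whose sphere color shows whether a planet is orbiting it.
; Every Tick it reads DoesHavePlanetOrbiting, creates a new dynamic instance of GoalStarMat and tints it cyan-blue if true, purple otherwise.
; A DidPlayAudio flag makes the Starhit sound play once at the world origin, on the first Tick regardless of orbit state.
; Nothing in this Blueprint sets the orbit flag.
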(event `self.ReceiveTick`
  (params (DeltaSeconds :type "Float (single-precision)"))
  (if (`self.doesHavePlanetOrbiting`)
    (bind _returnvalue (`PrimitiveComponent.CreateDynamicMaterialInstance` (`self.Sphere`) 0 "/Game/Materials/GoalStarMat.GoalStarMat" "None"))
    (`MaterialInstanceDynamic.SetVectorParameterValue` _returnvalue "Color" (make `LinearColor` 0.0 0.651 1.0 1.0))
    (else
      (bind _returnvalue_2 (`PrimitiveComponent.CreateDynamicMaterialInstance` (`self.Sphere`) 0 "/Game/Materials/GoalStarMat.GoalStarMat" "None"))
      (`MaterialInstanceDynamic.SetVectorParameterValue` _returnvalue_2 "Color" (make `LinearColor` 0.651 0.0 1.0 1.0))))
  (if (not (`self.didPlayAudio`))
    (`GameplayStatics.PlaySoundAtLocation` "/Game/Sound/starhit.starhit" (0.0 0.0 0.0) (struct) 1.0 1.0 0.0 null null null)
    (set `self.didPlayAudio` true)))

(fn `UserConstructionScript`)
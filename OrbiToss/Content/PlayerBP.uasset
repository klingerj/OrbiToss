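; VR player Blueprint that lets the left hand grab and throw planets.
; Overlaps on the hand Cube select a PlanetBP, which attaches on press with its force consideration disabled.
; Release re-enables force, throws it using the hand's scaled per-frame position delta, spawns an actor at a fixed spot and increments BallsUsed on the InteractiveWidget.
; The Cube1 overlap handlers are empty.
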(event `self.ReceiveTick`
  (params (DeltaSeconds :type "Float (single-precision)"))
  (bind _returnvalue (`SceneComponent.K2_GetComponentLocation` (`self.Cube`)))
  (set `self.LeftHandVelocity` (- _returnvalue (`self.LeftHandLastPos`)))
  (set `self.LeftHandLastPos` _returnvalue))

(event `self.ReceiveBeginPlay`
  (`HeadMountedDisplayFunctionLibrary.SetTrackingOrigin` "Floor")
  (set `self.LeftHandLastPos` (`SceneComponent.K2_GetComponentLocation` (`self.Cube`))))

(event `InputAction|LeftController`
  (params (Key :type "Key Structure"))
  (bind _currentplanet (`self.CurrentPlanet`))
  (bind _cube (`self.Cube`))
  (:`Pressed`
    (bind _asplanet_bp (cast `/Game/PlanetBP` _currentplanet))
    (`SceneComponent.K2_AttachToComponent` (`Actor.RootComponent` _asplanet_bp) _cube "None" "SnapToTarget" "SnapToTarget" "KeepWorld" true)
    (set `Planet.considerForce` false _asplanet_bp)
    (set `self.LeftHandFull` true))
  (:`Released`
    (bind _asplanet_bp_2 (cast `/Game/PlanetBP` _currentplanet))
    (`SceneComponent.K2_DetachFromComponent` (`Actor.RootComponent` _asplanet_bp_2) "KeepWorld" "KeepWorld" "KeepWorld" true)
    (set `self.LeftHandFull` false)
    (set `Planet.considerForce` true _asplanet_bp_2)
    (set `Planet.pos` (`SceneComponent.K2_GetComponentLocation` _cube) _asplanet_bp_2)
    (set `self.CurrentPlanet` self)
    (set `Planet.vel` (* (`self.LeftHandVelocity`) 80.0) _asplanet_bp_2)
    (`|SpawnActorFromClass` "/Game/PlanetBP.PlanetBP_C" (`KismetMathLibrary.MakeTransform` (-5.0 -10.0 140.0)) "AlwaysSpawn" "OverrideRootScale" null null)
    (bind _foundwidgets (`WidgetBlueprintLibrary.GetAllWidgetsOfClass` "/Game/InteractiveWidget.InteractiveWidget_C" false))
    (bind _output (`|GetArrayItem` _foundwidgets))
    (set `/Game/InteractiveWidget.BallsUsed` (+ (`/Game/InteractiveWidget.BallsUsed` _output) 1) _output)))

(event `self.Cube.OnComponentBeginOverlap`
  (params (OverlappedComponent :type "PrimitiveComponent Object Reference") (OtherActor :type "Actor Object Reference") (OtherComp :type "PrimitiveComponent Object Reference") (OtherBodyIndex :type Integer) (bFromSweep :type Boolean) (SweepResult :type "HitResult Structure (by ref)"))
  (if (not (`self.LeftHandFull`))
    (bind _asplanet_bp (cast `/Game/PlanetBP` OtherActor))
    (set `self.CurrentPlanet` _asplanet_bp)))

(event `self.Cube.OnComponentEndOverlap`
  (params (OverlappedComponent :type "PrimitiveComponent Object Reference") (OtherActor :type "Actor Object Reference") (OtherComp :type "PrimitiveComponent Object Reference") (OtherBodyIndex :type Integer))
  (if (not (`self.LeftHandFull`))
    (set `self.CurrentPlanet` self)))

(event `self.Cube1.OnComponentBeginOverlap`
  (params (OverlappedComponent :type "PrimitiveComponent Object Reference") (OtherActor :type "Actor Object Reference") (OtherComp :type "PrimitiveComponent Object Reference") (OtherBodyIndex :type Integer) (bFromSweep :type Boolean) (SweepResult :type "HitResult Structure (by ref)")))

(event `self.Cube1.OnComponentEndOverlap`
  (params (OverlappedComponent :type "PrimitiveComponent Object Reference") (OtherActor :type "Actor Object Reference") (OtherComp :type "PrimitiveComponent Object Reference") (OtherBodyIndex :type Integer)))

(fn `UserConstructionScript`)
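; LevelIndicationBP is an indicator actor that shows whether one of four levels has been completed.
; Every Tick, a branch chain on its Id (0 to 3) reads the matching completion flag from GiuseppesGameInstance.
; When that flag is set, it applies the TargetHit material to its Cylinder, repeating each frame rather than once.
; BeginPlay enables player input, though the graph contains no input events.
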(event `self.ReceiveTick`
  (params (DeltaSeconds :type "Float (single-precision)"))
  (if (== 0 (`self.id`))
    (bind _asgiuseppes_game_instance (cast `/Game/GiuseppesGameInstance` (`GameplayStatics.GetGameInstance`)))
    (if (`/Game/GiuseppesGameInstance.Level1Complete` _asgiuseppes_game_instance)
      (`PrimitiveComponent.SetMaterial` (`self.Cylinder`) 0 "/Game/Materials/TargetHit.TargetHit" :!label _label))
    (elif (== (`self.id`) 1)
      (bind _asgiuseppes_game_instance_2 (cast `/Game/GiuseppesGameInstance` (`GameplayStatics.GetGameInstance`)))
      (if (`/Game/GiuseppesGameInstance.Level2Complete` _asgiuseppes_game_instance_2)
        (goto _label))
      (elif (== (`self.id`) 2)
        (bind _asgiuseppes_game_instance_3 (cast `/Game/GiuseppesGameInstance` (`GameplayStatics.GetGameInstance`)))
        (if (`/Game/GiuseppesGameInstance.Level3Complete` _asgiuseppes_game_instance_3)
          (goto _label))
        (elif (== (`self.id`) 3)
          (bind _asgiuseppes_game_instance_4 (cast `/Game/GiuseppesGameInstance` (`GameplayStatics.GetGameInstance`)))
          (if (`/Game/GiuseppesGameInstance.Level4Complete` _asgiuseppes_game_instance_4)
            (goto _label)))))))

(event `self.ReceiveBeginPlay`
  (`self.EnableInput` (`GameplayStatics.GetPlayerController` 0)))

(fn `UserConstructionScript`)